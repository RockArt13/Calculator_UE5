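; Base actor component for calculator commands, which registers a command with the calculator component on the same owner.
; On BeginPlay it looks up BP_CalculatorComponent, pushes its name, displayed name and key through PushFullCommand, and stores the returned command.
; If no calculator is found, it deactivates itself and reports failure.
; RunCommand is an empty function, leaving the command's behavior to child Blueprints.
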(event EventBeginPlay
  (CallFunction|ConnecttoCalculator))

(fn ConnecttoCalculator
  (bind _returnvalue (Components|GetOwner))
  (bind _returnvalue_2 (Actor|GetComponentbyClass _returnvalue "/Game/Calculator/Core/BP_CalculatorComponent.BP_CalculatorComponent_C"))
  (Utilities|IsValid _returnvalue_2
    (:Is%20Valid
      (bind _output_get (Variables|Default|SetCalculatorComponent _returnvalue_2))
      (bind _command (Default|PushFullCommand _output_get (Variables|Default|GetCommandName) (Variables|Default|GetDisplayedName) (Variables|Default|GetKey)))
      (Variables|Default|SetCommand _command)
      (return true))
    (:Is%20Not%20Valid
      (Components|Activation|Deactivate)
      (return false))))

(fn RunCommand
  (params (Command :type BP%20Command%20Object%20Object%20Reference)))