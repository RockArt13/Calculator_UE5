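; Calculator command component for equals that executes the active commands held by the CalculatorComponent.
; Given a valid command, RunCommand pops active commands in a loop until none remains.
; It passes each to the first BP_SavedCommandComponent on its owner tagged with that command's name, skipping it if none is valid.
; Numeric command names all route to the component tagged "Number".
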(fn RunCommand
  (params (Command :type BP%20Command%20Object%20Object%20Reference))
  (Utilities|IsValid Command
    (:Is%20Valid
      (while true
        (bind _command (Default|PopActiveCommand (Variables|Default|GetCalculatorComponent)))
        (Utilities|IsValid _command
          (:Is%20Valid
            (Utilities|IsValid (Utilities|Array|Get(acopy) (Actor|GetComponentsbyTag (Components|GetOwner) "/Game/Calculator/Commands/BP_SavedCommandComponent.BP_SavedCommandComponent_C" (Utilities|String|StringToName (Utilities|String|SelectString "Number" (Variables|/Game/Calculator/Core/BP_CommandObject.BP_CommandObject_C|GetCommandName _command) (Class|KismetStringLibrary|IsNumeric (Variables|/Game/Calculator/Core/BP_CommandObject.BP_CommandObject_C|GetCommandName _command))))))
              (:Is%20Valid
                (CallFunction|RunCommand (Utilities|Array|Get(acopy) (Actor|GetComponentsbyTag (Components|GetOwner) "/Game/Calculator/Commands/BP_SavedCommandComponent.BP_SavedCommandComponent_C" (Utilities|String|StringToName (Utilities|String|SelectString "Number" (Variables|/Game/Calculator/Core/BP_CommandObject.BP_CommandObject_C|GetCommandName _command) (Class|KismetStringLibrary|IsNumeric (Variables|/Game/Calculator/Core/BP_CommandObject.BP_CommandObject_C|GetCommandName _command)))))) _command))))
          (:Is%20Not%20Valid
            (return) ; Cancels the loop
          ))))))