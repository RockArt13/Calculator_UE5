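; BP_NumberCommandTest is a functional test for the calculator's number command.
; It checks that the Calculator has a BP_NumberCommandComponent, then runs that component with a command object named after NumberTest and pops a value from the calculator component.
; The comparison of the popped value to NumberTest is unwired, so that step never reports pass or fail.
; StartTest finishes with a success result after both checks.
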(event EventPrepareTest
  (|CallParentFunction))

(event EventStartTest
  (|CallParentFunction)
  (|TestIfCommandIsValid)
  (|TestIfRunCommandWorked)
  (Class|FunctionalTest|FinishTest "Succeeded" "Passed Number Command Test"))

(fn ConstructionScript
  (|CallParentFunction))