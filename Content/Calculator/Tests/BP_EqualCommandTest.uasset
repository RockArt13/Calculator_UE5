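; Functional test for the calculator's Equal command component, run from StartTest as two checks in sequence.
; It first confirms the Calculator has a BP_EqualCommandComponent.
; It then seeds the UI's active command list with a ValueTest command, runs Equal with a second command object, and expects the display to equal ValueTest and the list to be empty.
; Either failed check finishes the test as Failed.
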(event EventPrepareTest
  (|CallParentFunction))

(event EventStartTest
  (|CallParentFunction)
  (|TestIfCommandIsValid)
  (|TestIfRunCommandWorked)
  (Class|FunctionalTest|FinishTest "Succeeded" "Passed Equal Command Test"))

(fn ConstructionScript
  (|CallParentFunction))