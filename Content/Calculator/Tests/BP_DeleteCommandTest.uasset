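; Functional test that checks the calculator's delete command.
; It first confirms the Calculator has a BP_DeleteCommandComponent.
; It then adds a "Del" command object to the UI's ActiveCommandList, runs the component with a second blank command object, and expects an empty list.
; Each check logs success or fails the test, and StartTest calls a success finish after both.
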(event EventPrepareTest
  (|CallParentFunction))

(event EventStartTest
  (|CallParentFunction)
  (|TestIfCommandIsValid)
  (|TestIfRunCommandWorked)
  (Class|FunctionalTest|FinishTest "Succeeded" "Passed Delete Command Test"))

(fn ConstructionScript
  (|CallParentFunction))