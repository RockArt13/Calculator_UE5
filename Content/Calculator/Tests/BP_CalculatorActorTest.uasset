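; Functional test that checks for the presence of a Calculator and its calculator component.
; PrepareTest calls the parent and starts a three-second Delay with nothing wired after it.
; StartTest validates the Calculator reference, then the BPCalculatorComponent reference, and finishes as Succeeded only if both are valid, otherwise Failed with a message naming the missing one.
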(event EventPrepareTest
  (|CallParentFunction)
  (Utilities|FlowControl|Delay 3.0))

(event EventStartTest
  (|CallParentFunction)
  (Utilities|IsValid (Variables|Default|GetCalculator)
    (:Is%20Valid
      (Class|FunctionalTest|LogMessage "Succeed to Find Calculator")
      (Utilities|IsValid (Variables|Default|GetBP%20Calculator%20Component)
        (:Is%20Valid
          (Class|FunctionalTest|FinishTest "Succeeded" "Succeed to Find Calculator Component"))
        (:Is%20Not%20Valid
          (Class|FunctionalTest|FinishTest "Failed" "Failed to Find Calculator Component"))))
    (:Is%20Not%20Valid
      (Class|FunctionalTest|FinishTest "Failed" "Failed to Find Calculator"))))

(fn ConstructionScript
  (|CallParentFunction))