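; Functional test for the Calculator Component that runs three checks in sequence on StartTest.
; It round-trips a value through push and pop, then pushes a full command and looks it up in the UI's full command list.
; That command is reused for the active-command push and pop, whose branch is always true because the field comparison is left unconnected.
; Failed checks finish the test as Failed.
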(event EventPrepareTest
  (|CallParentFunction) ; This node is disabled and will not be called.\nDrag off pins to build functionality.
)

(event EventStartTest
  (|CallParentFunction)
  (|TestPushPopValue)
  (|TestPushFullCommand)
  (|TestPushPopActiveCommand)
  (Class|FunctionalTest|FinishTest "Default" "Succeeded to test Calculator Component "))

(fn ConstructionScript
  (|CallParentFunction))