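; BP_Calculator is the calculator actor that hosts a BPCalculatorComponent and routes keyboard input to it.
; On BeginPlay the component creates the user interface and generates command components, and on EndPlay it removes the interface.
; Any key press is passed to the component for dynamic command lookup, playing a click sound when a command runs.
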(event EventBeginPlay
  ;[1 1 1] Create UserInterface and Generate Commands
  (Default|CreateUserInterface (Variables|Default|GetBP_CalculatorComponent))
  (Default|GenerateCommandComponents (Variables|Default|GetBP_CalculatorComponent)))

(event EventEndPlay
  (params (EndPlayReason :type EEndPlayReason%20Enum :default "Destroyed"))
  ;[1 1 1] Remove UserInterface
  (Default|RemoveUserInterface (Variables|Default|GetBP_CalculatorComponent)))

(event Input|KeyboardEvents|AnyKey
  (params (Key :type Key%20Structure))
  ;[1 1 1] Dynamic keyboard mapping
  (:Pressed
    (bind _issuccess (Default|RunCommandbyKey (Variables|Default|GetBP_CalculatorComponent) Key))
    (if _issuccess
      (Audio|PlaySound2D "/Engine/VREditor/Sounds/UI/Click_on_Button_Cue.Click_on_Button_Cue" 1.0 1.0 0.0 0 0))))

(fn ConstructionScript)