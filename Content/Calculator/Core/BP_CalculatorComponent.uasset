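; Calculator core component that owns the calculator widget, a value stack and the queue of active commands held in the UI list.
; Commands dispatch to tag-matched components on the owner: special ones run immediately, others are queued as command objects and later run by saved-command components, with numbers sharing one tag.
; It adds core command components and registers the owner with GameFrameworkComponentManager for feature extensions.
; Key lookup always returns false because its match logic is disconnected.
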(fn PopActiveCommand
  (if (> (Class|ListView|GetNumItems (Variables|/Game/Calculator/UI/WBP_Calculator.WBP_Calculator_C|GetActiveCommandList (Variables|Default|GetUserInterface))) 0)
    (bind _output_get (LocalVariables|SetTemporary (Class|ListView|GetItemat (Variables|/Game/Calculator/UI/WBP_Calculator.WBP_Calculator_C|GetActiveCommandList (Variables|Default|GetUserInterface)))))
    (Class|ListView|RemoveItem (Variables|/Game/Calculator/UI/WBP_Calculator.WBP_Calculator_C|GetActiveCommandList (Variables|Default|GetUserInterface)) _output_get)
    (bind _asbp_command_object (Utilities|Casting|CastToBP_CommandObject (LocalVariables|GetTemporary))
      (:then
        (return _asbp_command_object))
      (:CastFailed
        (return 0)))
    (else
      (return 0))))

(fn PushActiveCommand
  (params (Command :type BP%20Command%20Object%20Object%20Reference))
  (bind _userinterface (Variables|Default|GetUserInterface))
  (bind _inputtext (Variables|/Game/Calculator/UI/WBP_Calculator.WBP_Calculator_C|GetInputText _userinterface))
  (bind _returnvalue (Class|EditableTextBox|GetText _inputtext))
  (bind _returnvalue_2 (Utilities|String|ToString(Text) _returnvalue))
  ;[1 1 1] Dealing with Number comments
  (bind _output_get (LocalVariables|SetTemporary Command))
  (if (Utilities|Enum|NotEqual(Enum) (Variables|/Game/Calculator/Core/BP_CommandObject.BP_CommandObject_C|GetCommandName _output_get) "Number")
    (LocalVariables|SetName (Variables|/Game/Calculator/Core/BP_CommandObject.BP_CommandObject_C|GetCommandName (LocalVariables|GetTemporary)))
    (bind _returnvalue_3 (Game|ConstructObjectfromClass "/Game/Calculator/Core/BP_CommandObject.BP_CommandObject_C" self (LocalVariables|GetName) (Variables|/Game/Calculator/Core/BP_CommandObject.BP_CommandObject_C|GetDisplayedName (LocalVariables|GetTemporary)) (Variables|/Game/Calculator/Core/BP_CommandObject.BP_CommandObject_C|GetKey (LocalVariables|GetTemporary)) :!label _label))
    (Class|ListView|AddItem (Variables|/Game/Calculator/UI/WBP_Calculator.WBP_Calculator_C|GetActiveCommandList (Variables|Default|GetUserInterface)) _returnvalue_3)
    (else
      (LocalVariables|SetName _returnvalue_2)
      (if (Class|KismetStringLibrary|IsNumeric _returnvalue_2)
        (goto _label)))))

(fn PopValue
  (bind (_lastvalue _lastindex) (CallFunction|GetLastValue))
  (LocalVariables|SetTemporary _lastvalue)
  (Utilities|Array|RemoveIndex (Variables|Default|GetValueList) _lastindex)
  (bind _lastvalue_2 (CallFunction|GetLastValue))
  (Default|CallOnValueChanged _lastvalue_2)
  (return (LocalVariables|GetTemporary)))

(fn PushValue
  (params (Value :type Float%20%28single-precision%29))
  (Utilities|Array|Add (Variables|Default|GetValueList) Value)
  (Default|CallOnValueChanged Value))

(fn PushFullCommand
  (params (CommandName :type String) (DisplayedName :type String) (Key :type Key%20Structure :default "None"))
  (bind _returnvalue (Game|ConstructObjectfromClass "/Game/Calculator/Core/BP_CommandObject.BP_CommandObject_C" self CommandName DisplayedName Key))
  (Class|ListView|AddItem (Variables|/Game/Calculator/UI/WBP_Calculator.WBP_Calculator_C|GetFullComandList (Variables|Default|GetUserInterface)) _returnvalue)
  (return _returnvalue))

(fn GetLastValue
  (bind _valuelist (Variables|Default|GetValueList))
  (bind _returnvalue (Utilities|Array|LastIndex _valuelist))
  (return (Utilities|Array|Get(acopy) _valuelist _returnvalue) _returnvalue))

(fn ValueChanged
  (params (Value :type Float%20%28single-precision%29))
  (Variables|/Game/Calculator/UI/WBP_Calculator.WBP_Calculator_C|SetText (Variables|Default|GetUserInterface) (Utilities|String|ToString(Float) Value)))

(fn RunCommandbyKey
  (params (Key :type Key%20Structure :default "None"))
  (for _array_element (Class|ListView|GetListItems (Variables|/Game/Calculator/UI/WBP_Calculator.WBP_Calculator_C|GetFullComandList (Variables|Default|GetUserInterface)))
    _)
  (return false))

(fn RunCommandSpecial
  (params (Command :type BP%20Command%20Object%20Object%20Reference))
  (bind _output_get (LocalVariables|SetTemporary Command))
  (if (Utilities|Array|IsValidIndex (Actor|GetComponentsbyTag (Components|GetOwner) "/Game/Calculator/Commands/BP_SpecialCommandComponent.BP_SpecialCommandComponent_C" (Utilities|String|StringToName (Variables|/Game/Calculator/Core/BP_CommandObject.BP_CommandObject_C|GetCommandName _output_get))))
    (Default|RunCommand (Utilities|Array|Get(acopy) (Actor|GetComponentsbyTag (Components|GetOwner) "/Game/Calculator/Commands/BP_SpecialCommandComponent.BP_SpecialCommandComponent_C" (Utilities|String|StringToName (Variables|/Game/Calculator/Core/BP_CommandObject.BP_CommandObject_C|GetCommandName _output_get)))) (LocalVariables|GetTemporary))
    (else
      (CallFunction|PushActiveCommand (LocalVariables|GetTemporary)))))

(fn RunCommandSaved
  (bind _command (CallFunction|PopActiveCommand))
  (LocalVariables|SetTemporary _command)
  (Utilities|IsValid (Utilities|Array|Get(acopy) (Actor|GetComponentsbyTag (Components|GetOwner) "/Game/Calculator/Commands/BP_SavedCommandComponent.BP_SavedCommandComponent_C" (Utilities|String|StringToName (Utilities|String|SelectString "Number" (Variables|/Game/Calculator/Core/BP_CommandObject.BP_CommandObject_C|GetCommandName _command) (Class|KismetStringLibrary|IsNumeric (Variables|/Game/Calculator/Core/BP_CommandObject.BP_CommandObject_C|GetCommandName _command))))))
    (:Is%20Valid
      (Default|RunCommand (Utilities|Array|Get(acopy) (Actor|GetComponentsbyTag (Components|GetOwner) "/Game/Calculator/Commands/BP_SavedCommandComponent.BP_SavedCommandComponent_C" (Utilities|String|StringToName (Utilities|String|SelectString "Number" (Variables|/Game/Calculator/Core/BP_CommandObject.BP_CommandObject_C|GetCommandName _command) (Class|KismetStringLibrary|IsNumeric (Variables|/Game/Calculator/Core/BP_CommandObject.BP_CommandObject_C|GetCommandName _command)))))) (LocalVariables|GetTemporary))
      (return true))
    (:Is%20Not%20Valid
      (return false))))

(fn CreateUserInterface
  (bind _returnvalue (UserInterface|CreateWidget "/Game/Calculator/UI/WBP_Calculator.WBP_Calculator_C" (Game|GetPlayerController 0)))
  (bind _output_get (Variables|Default|SetUserInterface _returnvalue))
  (UserInterface|Viewport|AddtoViewport _output_get 0)
  (Variables|/Script/Engine.PlayerController|SetbShowMouseCursor (Game|GetPlayerController 0) false)
  (EventDispatchers|BindEventtoOnCommandDispatched (Variables|Default|GetUserInterface) (EventDispatchers|CreateEvent :!event RunCommandSpecial))
  (EventDispatchers|BindEventtoOnValueChanged (EventDispatchers|CreateEvent :!event ValueChanged))
  (return))

(fn RemoveUserInterface
  (Widget|RemovefromParent (Variables|Default|GetUserInterface)))

(fn GenerateCommandComponents
  (for _array_element (Variables|Default|GetCoreCommands)
    (Game|AddComponentbyClass (Components|GetOwner) _array_element))
  ;[1 1 1] Connect to Features
  (Class|GameFrameworkComponentManager|AddReceiver (Subsystems|GetGameFrameworkComponentManager) (Components|GetOwner)))